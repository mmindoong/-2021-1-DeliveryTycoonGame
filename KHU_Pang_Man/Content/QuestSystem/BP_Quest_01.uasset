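; Quest Blueprint for "A Long Way Home", which tasks the player with reaching Megaton.
; It builds an order-required BP_ObjReach as the root objective through ConstructRootObjectiveReach.
; PopulateObjectives adds a single BP_ObjReachDestination child, "Reach Megaton", to the passed-in root, with MegatonTrigger as its destination.
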(fn `ConstructRootObjectiveReach`
  (returns (RootObjReach :type "/Game/QuestSystem/BP_ObjReach Object Reference"))
  (bind _returnvalue (`|GenericCreateObject` "/Game/QuestSystem/BP_ObjReach.BP_ObjReach_C" self true "A Long Way Home"))
  (return _returnvalue))

(fn `PopulateObjectives`
  (params (RootObjReachs :type "/Game/QuestSystem/BP_ObjReach Object Reference"))
  (returns (RootObjReach :type "/Game/QuestSystem/BP_ObjReach Object Reference"))
  (bind _returnvalue (`|GenericCreateObject` "/Game/QuestSystem/BP_ObjReachDestination.BP_ObjReachDestination_C" self (`self.Megaton Trigger`) "Reach Megaton"))
  (`/Game/QuestSystem/BP_ObjReach.AddObjective` (`local.RootObjReachs`) _returnvalue))

(fn `UserConstructionScript`
  (`parent.UserConstructionScript`))