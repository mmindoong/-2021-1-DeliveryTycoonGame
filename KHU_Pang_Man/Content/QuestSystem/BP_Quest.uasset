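; BP_Quest is a base quest Blueprint that sets up and starts a quest's objectives.
; On BeginPlay it builds and stores a root objective collection, populates it, then activates it.
; The construct and populate functions are stubs that print an error, so child quests are expected to override them.
; A getter exposes the root collection.
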(event `self.ReceiveBeginPlay`
  (bind _rootobjreach (`self.ConstructRootObjectiveReach`))
  (bind _output_get (set `self.RootObjCollection` _rootobjreach))
  (`self.PopulateObjectives` _output_get)
  (`/Game/QuestSystem/BP_Ojective.ActivateObjective` (`self.RootObjCollection`)))

(fn `ConstructRootObjectiveReach`
  (returns (RootObjReach :type "/Game/QuestSystem/BP_ObjReach Object Reference"))
  (`KismetSystemLibrary.PrintString` "Error : CreateRootObjectiveReach called for base class")
  (return null))

(fn `GetRootObjectiveReach`
  (returns (RootObjReachDestination :type "/Game/QuestSystem/BP_ObjReach Object Reference"))
  (return (`self.RootObjCollection`)))

(fn `PopulateObjectives`
  (params (RootObjReachs :type "/Game/QuestSystem/BP_ObjReach Object Reference"))
  (returns (RootObjReach :type "/Game/QuestSystem/BP_ObjReach Object Reference"))
  (`KismetSystemLibrary.PrintString` "Error : PopulatebjectiveReach called for base class")
  (return null))

(fn `UserConstructionScript`)